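; Actor Blueprint for a whack-a-mole mole that pops up and down through the PopUpnDown level sequence, rewound to frame zero on BeginPlay.
; BeginSpawn waits a random delay, plays the sequence, sets IsActive for a short window, then calls itself to loop.
; Whacked plays the sequence in reverse, clears IsWhacked immediately, then after a delay sets IsActive and re-enters BeginSpawn.
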(event Custom|BeginSpawn
  (if (not (Variables|Default|GetIsWhacked))
    (Utilities|FlowControl|Delay (Math|Random|RandomFloatinRange 0.5 3.5))
    (if (not (Variables|Default|GetIsWhacked))
      (Sequencer|Player|Play (Variables|/Script/ActorSequence.ActorSequenceComponent|GetSequencePlayer (Variables|Default|GetPopUpnDown)) :!class /Script/MovieScene.MovieSceneSequencePlayer)
      (Variables|Default|SetIsActive true)
      (Utilities|FlowControl|Delay 0.7)
      (Variables|Default|SetIsActive false)
      (Utilities|FlowControl|Delay 0.5)
      (CallFunction|BeginSpawn))))

(event Custom|Whacked
  (Variables|Default|SetIsWhacked true)
  (Variables|Default|SetIsActive false)
  (Class|MovieSceneSequencePlayer|PlayReverse (Variables|/Script/ActorSequence.ActorSequenceComponent|GetSequencePlayer (Variables|Default|GetPopUpnDown)))
  (Variables|Default|SetIsWhacked false)
  (Utilities|FlowControl|Delay 0.6)
  (Variables|Default|SetIsActive true)
  (CallFunction|BeginSpawn))

(event EventBeginPlay
  ;[1 1 1] Event Begin
  (Components|Timeline|SetPlaybackPosition (Variables|/Script/ActorSequence.ActorSequenceComponent|GetSequencePlayer (Variables|Default|GetPopUpnDown)) (Utilities|Struct|MakeMovieSceneSequencePlaybackParams (Utilities|Struct|MakeFrameTime (Utilities|Struct|MakeFrameNumber) 0.0) 0.0 "" "Frame" "Play")))

(event Collision|EventActorBeginOverlap
  (params (OtherActor :type Actor%20Object%20Reference)))

(event EventTick
  (params (DeltaSeconds :type Float%20%28single-precision%29)))

(fn ConstructionScript)